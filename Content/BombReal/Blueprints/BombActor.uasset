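; Bomb actor that signals its countdown through its material, then destroys itself.
; BeginPlay puts a dynamic material instance on the static mesh and raises its Frequency parameter in steps across shrinking delays before DestroyActor.
; The graph spawns no explosion effect and applies no damage.
; An unconnected timer-driven Lerp of the same parameter, with a debug print, never runs.
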(event `self.ReceiveBeginPlay`
  (bind _dynamicmaterial (`self.DynamicMaterial`))
  (bind _returnvalue (`KismetMaterialLibrary.CreateDynamicMaterialInstance` "/Game/BombReal/BombMaterial.BombMaterial"))
  (bind _output_get (set `self.DynamicMaterial` _returnvalue))
  (`PrimitiveComponent.SetMaterial` (`self.StaticMesh`) 0 _output_get)
  ;[1 1 1] Play effects before exploding
  (`MaterialInstanceDynamic.SetScalarParameterValue` _dynamicmaterial "Frequency" 2.0)
  (`KismetSystemLibrary.Delay` 2.0)
  (`MaterialInstanceDynamic.SetScalarParameterValue` _dynamicmaterial "Frequency" 5.0)
  (`KismetSystemLibrary.Delay` 1.0)
  (`MaterialInstanceDynamic.SetScalarParameterValue` _dynamicmaterial "Frequency" 10.0)
  (`KismetSystemLibrary.Delay` 0.5)
  (`self.K2_DestroyActor`))

(event `self.ReceiveTick`
  (params (DeltaSeconds :type "Float (single-precision)")))

(event `CustomEvent_0`)

(fn `UserConstructionScript`)