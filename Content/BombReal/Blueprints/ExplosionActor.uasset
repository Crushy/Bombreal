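; ExplosionActor is a short-lived explosion actor that destroys itself half a second after spawning.
; On overlap, it detonates any BombActor it touches, setting off chain reactions between bombs.
; It also kills any overlapping TopDownCharacter by destroying the actor outright.
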(event `self.ReceiveBeginPlay`
  (`KismetSystemLibrary.Delay` 0.5)
  (`self.K2_DestroyActor`))

(event `self.ReceiveActorBeginOverlap`
  (params (OtherActor :type "Actor Object Reference"))
  (`|ExecutionSequence`
    (:`then_0`
      ;[1 1 1] If other bomb, detonate it imediately
      (bind _asbomb_actor (cast `/Game/BombReal/Blueprints/BombActor` OtherActor))
      (`/Game/BombReal/Blueprints/BombActor.Detonate` _asbomb_actor))
    (:`then_1`
      ;[1 1 1] If player, kill him
      (bind _astop_down_character (cast `/Game/BombReal/Blueprints/TopDownCharacter` OtherActor))
      (`self.K2_DestroyActor` _astop_down_character))))

(fn `UserConstructionScript`)