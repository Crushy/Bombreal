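; Shared camera actor that frames every Character in the level in one view, set as the view target of all player controllers at BeginPlay.
; Each tick it re-gathers all Characters and moves itself to their average location.
; It then sets the camera arm length from the furthest Character's distance scaled by the cosine of half the FOV, plus padding, with a clamped minimum.
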(event `self.ReceiveBeginPlay`
  ;[1 1 1] Not needed but just to be sure, set all players to use this camera
  (bind _outactors (`GameplayStatics.GetAllActorsOfClass` "/Script/Engine.PlayerController"))
  (`PlayerController.SetViewTargetWithBlend` _outactors self 0.0 "VTBlend_Linear" 0.0 false)
  (bind _outactors_2 (`GameplayStatics.GetAllActorsOfClass` "/Script/Engine.Character"))
  (set `self.AllFocusedActors` _outactors_2))

(event `self.ReceiveTick`
  (params (DeltaSeconds :type "Float (single-precision)"))
  (bind _allfocusedactors (`self.AllFocusedActors`))
  (bind _averagepoint (`self.AveragePoint`))
  (bind _outactors (`GameplayStatics.GetAllActorsOfClass` "/Script/Engine.Character"))
  (set `self.AllFocusedActors` _outactors)
  (set `self.AveragePoint` (0.0 0.0 0.0))
  (for _array_element _allfocusedactors
    (set `self.AveragePoint` (+ (`self.AveragePoint`) (`self.K2_GetActorLocation` _array_element))))
  (set `self.AveragePoint` (/ _averagepoint (`KismetArrayLibrary.Array_Length` _allfocusedactors)))
  (`self.K2_SetActorLocation` _averagepoint)
  (`self.FindFurthestPlayerFromCamera`))

(fn `FindFurthestPlayerFromCamera`
  (locals (NewLocalVar_0 :type "Actor Object Reference") (GreatestDistance :type "Float (double-precision)" :default 0.0))
  (set `local.GreatestDistance` 0.0)
  (for _array_element (`self.AllFocusedActors`)
    (bind _returnvalue (`KismetMathLibrary.VSize` (- (`self.K2_GetActorLocation` _array_element) (`self.AveragePoint`))))
    (if (> _returnvalue (`local.GreatestDistance`))
      (set `local.GreatestDistance` _returnvalue)
      (set `local.NewLocalVar_0` _array_element)))
  (set `SpringArmComponent.TargetArmLength` (`KismetMathLibrary.FClamp` (+ (* (`KismetMathLibrary.DegCos` (/ (`CameraComponent.FieldOfView` (`self.Camera`)) 2.0)) (`local.GreatestDistance`)) 1000.0) 1000.0 100000000.0) (`self.CameraArm`)))

(fn `UserConstructionScript`)