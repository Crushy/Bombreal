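; PowerUpBase is a pickup that grants a TopDownCharacter a random bomb or movement upgrade.
; The construction script picks a random PowerupType from the enum and labels the text render with a matching symbol.
; On overlap with the character, it raises bomb radius, max bombs or walk speed (clamped to a limit), then destroys itself.
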(event `self.ReceiveActorBeginOverlap`
  (params (OtherActor :type "Actor Object Reference"))
  (bind _astop_down_character (cast `/Game/BombReal/Blueprints/TopDownCharacter` OtherActor))
  (`|ExecutionSequence`
    (:`then_0`
      (switch `/Game/BombReal/Blueprints/PowerupTypesEnum` (`self.Powerup Type`)
        (:`NewEnumerator0`
          (`/Engine/EditorBlueprintResources/StandardMacros.IncrementInt` (`/Game/BombReal/Blueprints/TopDownCharacter.Bomb radius` _astop_down_character)))
        (:`NewEnumerator1`
          (`/Engine/EditorBlueprintResources/StandardMacros.IncrementInt` (`/Game/BombReal/Blueprints/TopDownCharacter.Max bombs` _astop_down_character)))
        (:`NewEnumerator2`
          (bind _charactermovement (`Character.CharacterMovement` _astop_down_character))
          (set `CharacterMovementComponent.MaxWalkSpeed` (`KismetMathLibrary.FClamp` (+ (`MovementComponent.GetMaxSpeed` _charactermovement) 500.0) 0.0 4000.0) _charactermovement))))
    (:`then_1`
      (`self.K2_DestroyActor`))))

(fn `UserConstructionScript`
  (bind _output_get (set `self.Powerup Type` (cast `/Game/BombReal/Blueprints/PowerupTypesEnum` (`KismetMathLibrary.Conv_IntToByte` (`KismetMathLibrary.RandomInteger` (enumcount `/Game/BombReal/Blueprints/PowerupTypesEnum`))))))
  (`TextRenderComponent.K2_SetText` (`self.TextRender`) (select `/Game/BombReal/Blueprints/PowerupTypesEnum` _output_get :`NewEnumerator0` "+" :`NewEnumerator1` "B" :`NewEnumerator2` "M" :!type "Text")))